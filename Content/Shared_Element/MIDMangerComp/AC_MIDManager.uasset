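; AC_MIDManager is a component with a function that swaps a mesh's material slot for a dynamic material instance.
; ReplaceDynamicMaterial creates the instance from the slot's base material rather than the assigned material, applies it to the slot and returns it.
; When flagged HasBarrior, the new instance is also collected in the BarriorMatInsDyns array.
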(event EventBeginPlay)

(event EventTick
  (params (DeltaSeconds :type Float%20%28single-precision%29)))

(fn ReplaceDynamicMaterial
  (params (TargetMesh :type Mesh%20Component%20Object%20Reference) (MatSlotIndex :type Integer) (HasBarrior :type Boolean))
  (bind _output_get (LocalVariables|SetMesh TargetMesh))
  (bind _returnvalue (Rendering|Material|GetBaseMaterial (Rendering|Material|GetMaterial _output_get MatSlotIndex)))
  (bind _returnvalue_2 (Rendering|Material|CreateDynamicMaterialInstance _returnvalue "None" "None" :!class /Script/Engine.KismetMaterialLibrary))
  (bind _output_get_2 (LocalVariables|SetDynamicMat _returnvalue_2))
  (Rendering|Material|SetMaterial (LocalVariables|GetMesh) MatSlotIndex _output_get_2)
  (if HasBarrior
    (Utilities|Array|Add (Variables|Default|GetBarriorMatInsDyns) (LocalVariables|GetDynamicMat)))
  (return (LocalVariables|GetDynamicMat)))