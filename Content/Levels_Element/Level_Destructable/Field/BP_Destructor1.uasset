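; BP_Destructor1 is a Chaos field actor that applies a disable-threshold physics field within a spherical area.
; Every Tick, a linear radial falloff built from the Sphere's world location and scaled radius, with FieldMagnitude as strength, feeds ApplyPhysicsField on the FieldSystemComponent.
; BeginPlay, Hit and the construction script are empty, and a delayed re-apply branch is left unconnected.
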(event EventBeginPlay)

(event Collision|EventActorBeginOverlap
  (params (OtherActor :type Actor%20Object%20Reference)))

(event EventTick
  (params (DeltaSeconds :type Float%20%28single-precision%29))
  (bind _sphere (Variables|Default|GetSphere))
  (Class|FieldSystemComponent|ApplyPhysicsField (Variables|Field|GetFieldSystemComponent) true "Field_DisableThreshold" 0 (Field|SetRadialFalloff (Variables|Default|GetRadialFalloff) (Variables|Default|GetField%20Magnitude) 0.0 1.0 0.0 (Components|Sphere|GetScaledSphereRadius _sphere) (Transformation|GetWorldLocation _sphere) "Field_Falloff_Linear")))

(event Collision|EventHit
  (params (MyComp :type Primitive%20Component%20Object%20Reference) (Other :type Actor%20Object%20Reference) (OtherComp :type Primitive%20Component%20Object%20Reference) (bSelfMoved :type Boolean) (HitLocation :type Vector :default "0, 0, 0") (HitNormal :type Vector :default "0, 0, 0") (NormalImpulse :type Vector :default "0, 0, 0") (Hit :type Hit%20Result%20Structure%20%28by%20ref%29)))

(fn ConstructionScript)