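; BP_SimpleDisableField is a field system actor that applies a persistent disable-threshold physics field to destructible simulation inside a box volume.
; On BeginPlay it clears existing persistent fields, then registers a disable-threshold field with a very high magnitude and no falloff.
; A culling field built from the same box transform restricts the effect to the box by culling everything outside it.
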(event EventBeginPlay
  (bind _fieldsystemcomponent (Variables|Field|GetFieldSystemComponent))
  (Utilities|FlowControl|Sequence
    (:then_0
      (Class|FieldSystemComponent|RemovePersistentFields _fieldsystemcomponent)
      (Class|FieldSystemComponent|AddPersistentField _fieldsystemcomponent true "Field_DisableThreshold" 0 (Field|SetCullingField (Variables|Default|GetCullingField) (Field|SetBoxFalloff (Variables|Default|GetBoxFalloff-Culling) 1.0 0.0 1.0 0.0 (Transformation|GetWorldTransform (Variables|Default|GetBox)) "Field_FallOff_None") (Field|SetBoxFalloff (Variables|Default|GetBoxFalloff) 5e+05 0.0 1.0 0.0 (Transformation|GetWorldTransform (Variables|Default|GetBox)) "Field_FallOff_None") "Field_Culling_Outside")))))

(event Collision|EventActorBeginOverlap
  (params (OtherActor :type Actor%20Object%20Reference)))

(event EventTick
  (params (DeltaSeconds :type Float%20%28single-precision%29)))

(fn ConstructionScript)