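; Actor component for a magic barrier that stores its max and current gauge and drives the barrier's look.
; InitBarrior fills the gauge; SetBarrior updates it and pushes parameters to the supplied dynamic material instances.
; Max gauge sets a sky-blue-to-purple color lerp, shape changes write the forward vector, and stat changes set intensity from the remaining fraction.
; GuageToStage, meant to convert gauge to stage, contains only an unconnected log2 node.
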(event EventBeginPlay
  (Variables|Default|SetCurrentGuage (Variables|Default|GetMaxGuage)))

(event EventTick
  (params (DeltaSeconds :type Float%20%28single-precision%29)))

(fn SetBarriorMatDynIns
  (params (TargetMatInsDyns :type Array%20of%20Material%20Instance%20Dynamic%20Object%20References) (IsChangeShape :type Boolean) (IsChangeStat :type Boolean) (ForwardVector :type Vector) (LeftGuagePercentage :type Float%20%28double-precision%29) (MaxGuage :type Float%20%28double-precision%29))
  (for _array_element TargetMatInsDyns
    (LocalVariables|SetTargetMatInsD _array_element)
    (Utilities|FlowControl|Sequence
      (:then_0
        ;[1 1 1] Max게이지가 0이면 하늘 1024면 보라색
        (Rendering|Material|SetScalarParameterValue (LocalVariables|GetTargetMatInsD) "ColorLerp" (/ (Utilities|GuagetoStage (Variables|Default|GetMaxGuage)) 1e+01) :!class /Script/Engine.MaterialInstanceDynamic))
      (:then_1
        ;[1 1 1] Shape ( 주로 polymorph 혹은 scale change )가 바뀔때 변하는 material param
        (if IsChangeShape
          (Rendering|Material|SetVectorParameterValue (LocalVariables|GetTargetMatInsD) "OSForwardVector" (Utilities|Struct|MakeLinearColor (.x ForwardVector) (.y ForwardVector) (.z ForwardVector) 0.0) :!class /Script/Engine.MaterialInstanceDynamic)))
      (:then_2
        ;[1 1 1] Stat ( 주로 저항강도 )가 바뀔때 변하는 material param
        (if IsChangeStat
          (Rendering|Material|SetScalarParameterValue (LocalVariables|GetTargetMatInsD) "BarriorIntensity" (Utilities|GuagetoStage (* LeftGuagePercentage 1024.0)) :!class /Script/Engine.MaterialInstanceDynamic))))))

(fn SetBarrior
  (params (TargetMatInsDyns :type AC%20MID%20Manager%20Object%20Reference) (IsChangeShape :type Boolean) (IsChangeStat :type Boolean) (ForwardVector :type Vector) (LeftGuage :type Float%20%28double-precision%29))
  (Utilities|FlowControl|Sequence
    (:then_0
      (Variables|Default|SetCurrentGuage LeftGuage))
    (:then_1
      (CallFunction|SetBarriorMatDynIns (Variables|/Game/Shared_Element/MIDMangerComp/AC_MIDManager.AC_MIDManager_C|GetBarriorMatInsDyns TargetMatInsDyns) IsChangeShape IsChangeStat ForwardVector (/ (Variables|Default|GetCurrentGuage) (Variables|Default|GetMaxGuage)) (Variables|Default|GetMaxGuage)))))

(fn InitBarrior
  (params (MIDManager :type AC%20MID%20Manager%20Object%20Reference) (IsChangeShape :type Boolean) (IsChangeStat :type Boolean) (ForwardVector :type Vector) (MaxGuage :type Float%20%28double-precision%29))
  (Utilities|FlowControl|Sequence
    (:then_0
      (bind _output_get (Variables|Default|SetMaxGuage MaxGuage))
      (Variables|Default|SetCurrentGuage _output_get))
    (:then_1
      (CallFunction|SetBarrior MIDManager IsChangeShape IsChangeStat ForwardVector MaxGuage))))