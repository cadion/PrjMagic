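; BP_MBDrgon is a dragon Barrior pawn for the magic barrier level element, set up with a magic barrier that can change shape and stat.
; The construction script has MIDManager swap the mesh's first material for a barrier-enabled dynamic material, then passes that manager to MagicBarriorComponent with a forward vector and max gauge.
; Tick draws a red debug box around the actor's bounds every frame.
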(event EventBeginPlay
  (|CallParentFunction) ; This node is disabled and will not be called.\nDrag off pins to build functionality.
)

(event Collision|EventActorBeginOverlap
  (params (OtherActor :type Actor%20Object%20Reference))
  (|CallParentFunction OtherActor) ; This node is disabled and will not be called.\nDrag off pins to build functionality.
)

(event EventTick
  (params (DeltaSeconds :type Float%20%28single-precision%29))
  (bind _self self)
  (bind (_origin _boxextent) (Collision|GetActorBounds _self false false))
  (|CallParentFunction DeltaSeconds)
  (Rendering|Debug|DrawDebugBox _origin _boxextent "(R=1.000000,G=0.000000,B=0.000000,A=1.000000)" "0, 0, 0" -1.0 1e+01))

(fn ConstructionScript
  (|CallParentFunction)
  (Utilities|FlowControl|Sequence
    (:then_0
      (Default|ReplaceDynamicMaterial (Variables|Default|GetMIDManager) (Variables|Character|GetMesh) 0 true))
    (:then_1
      (Default|InitBarrior (Variables|Default|GetMagicBarriorComponent) (Variables|Default|GetMIDManager) true true "0.000000,-1.000000,-1.000000" 512.0))))