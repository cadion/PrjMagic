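; Character Blueprint for magic barrier pawns, providing a helper for swapping mesh materials to dynamic instances.
; ReplaceDynamicMaterial builds a dynamic instance from a slot's root base material, rather than the assigned material instance, then applies it to that slot and returns it.
; Instances flagged as having a barrier are also collected in BarriorMatInsDyns.
; The event graph and construction script are empty.
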(event EventBeginPlay)

(event Collision|EventActorBeginOverlap
  (params (OtherActor :type Actor%20Object%20Reference)))

(event EventTick
  (params (DeltaSeconds :type Float%20%28single-precision%29)))

(fn ConstructionScript)

(fn ReplaceDynamicMaterial
  (params (MatSlotIndex :type Integer) (HasBarrior :type Boolean))
  (bind _returnvalue (Rendering|Material|GetBaseMaterial (Rendering|Material|GetMaterial (Variables|Character|GetMesh) MatSlotIndex)))
  (bind _returnvalue_2 (Rendering|Material|CreateDynamicMaterialInstance _returnvalue "None" "None" :!class /Script/Engine.KismetMaterialLibrary))
  (bind _output_get (LocalVariables|SetDynamicMat _returnvalue_2))
  (Rendering|Material|SetMaterial (Variables|Character|GetMesh) MatSlotIndex _output_get)
  (if HasBarrior
    (Utilities|Array|Add (Variables|Default|GetBarriorMatInsDyns) (LocalVariables|GetDynamicMat)))
  (return (LocalVariables|GetDynamicMat)))